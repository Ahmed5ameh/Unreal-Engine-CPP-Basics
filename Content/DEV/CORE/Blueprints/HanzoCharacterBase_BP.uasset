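; Base character Blueprint for Hanzo that sets up the on-screen UI and keeps the health display current.
; On BeginPlay it creates the crosshair and HUD widgets, adds them to the viewport and seeds the HUD from HealthComponentGDESS.
; AnyDamage pushes health to the HUD as an event-driven update, avoiding a per-frame property binding.
; TraceForward only calls the parent implementation.
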(event `self.TraceForward`
  (`parent.TraceForward`))

(event `self.ReceiveBeginPlay`
  (bind _healthcomponent_gdess (`self.HealthComponent_GDESS`))
  (bind _returnvalue (`|CreateWidget` "/Game/DEV/CORE/Blueprints/Widgets/Crosshair_WBP.Crosshair_WBP_C"))
  (`UserWidget.AddToViewport` _returnvalue 0)
  (bind _returnvalue_2 (`|CreateWidget` "/Game/DEV/CORE/Blueprints/Widgets/Hud_WBP.Hud_WBP_C"))
  (bind _output_get (set `self.HudRef` _returnvalue_2))
  (`UserWidget.AddToViewport` _output_get 0)
  (`/Game/DEV/CORE/Blueprints/Widgets/Hud_WBP.UpdateHealth` (`self.HudRef`) (`HealthComponent_GDESS.Health` _healthcomponent_gdess) (`HealthComponent_GDESS.MaxHealth` _healthcomponent_gdess)))

(event `self.ReceiveAnyDamage`
  (params (Damage :type "Float (single-precision)") (DamageType :type "DamageType Object Reference") (InstigatedBy :type "Controller Object Reference") (DamageCauser :type "Actor Object Reference"))
  (bind _healthcomponent_gdess (`self.HealthComponent_GDESS`))
  ;[0 0 0] This will update the "HUD_WDP" only once, instead of looping using the other methos where you bind the percentage to a function
  (`/Engine/EditorBlueprintResources/StandardMacros.IsValid` _healthcomponent_gdess
    (:`Is Valid`
      (`/Game/DEV/CORE/Blueprints/Widgets/Hud_WBP.UpdateHealth` (`self.HudRef`) (`HealthComponent_GDESS.Health` _healthcomponent_gdess) (`HealthComponent_GDESS.MaxHealth` _healthcomponent_gdess)))))

(fn `UserConstructionScript`)